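; Watering robot that receives tasks from BP_GameInstance and tends BP_Crop actors.
; On BeginPlay it binds to the task-assigned event, then for tasks matching its RobotId it AI-moves to the target, cycling RobotState with a three-second pause on arrival.
; DoWork separately runs WaterTask, which finds the crop by CropId, raises a clamped WaterLevel and clears the task.
; The move sequence never calls DoWork.
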(event `DoWork`
  (switch `/Game/Datas/Enum/E_TaskType` "NewEnumerator0"
    (:`NewEnumerator0`
      (`self.WaterTask`))))

(event `self.ReceiveBeginPlay`
  (bind _gameinstance (`self.GameInstanceCasting`))
  (add `/Game/Settings/BP_GameInstance.OnTaskAssinged` _gameinstance (delegate `OnTaskRecived`)))

(event `OnTaskRecived`
  (params (TaskData :type "/Game/Datas/Struct/ST_Task Structure"))
  (bind (_taskid _tasktype _assingedrobotid _targetlocation) (break `/Game/Datas/Struct/ST_Task` TaskData))
  (if (== _assingedrobotid (`self.RobotId`))
    (set `self.TargetLocation` _targetlocation)
    (set `self.RobotState` "NewEnumerator1")
    (`|AIMoveTo` self (`self.TargetLocation`) null
      (:`then`
        (set `self.RobotState` "NewEnumerator2")
        (`KismetSystemLibrary.Delay` 3.0)
        (set `self.RobotState` "NewEnumerator0")))))

(fn `GameInstanceCasting`
  (returns (GameInstance :type "/Game/Settings/BP_GameInstance Object Reference"))
  (bind _asbp_game_instance (cast `/Game/Settings/BP_GameInstance` (`GameplayStatics.GetGameInstance`)))
  (return _asbp_game_instance))

(fn `UserConstructionScript`)

(fn `WaterTask`
  (bind (_currenttask_taskid _currenttask_tasktype _currenttask_assingedrobotid _currenttask_targetlocation _currenttask_targetfloor _currenttask_targetshelf _currenttask_taskstate _currenttask_targetcropid) (break `/Game/Datas/Struct/ST_Task` (`self.CurrentTask`)))
  (bind _outactors (`GameplayStatics.GetAllActorsOfClass` "/Game/BluePrints/BP_Crop.BP_Crop_C"))
  (for _array_element _outactors
    (if (== (`/Game/BluePrints/BP_Crop.CropId` _array_element) _currenttask_targetcropid)
      (set `self.TargetCrop` _array_element)
      (for _ _ :!via `Break`
        _)))
  (`/Engine/EditorBlueprintResources/StandardMacros.IsValid` (`self.TargetCrop`)
    (:`Is Valid`
      (if true
        (set `self.WaterLevel` (`KismetMathLibrary.FClamp` (+ (`self.WaterLevel`) 0.3)))
        (`KismetSystemLibrary.PrintString` "waa")
        (set `self.HasTask` false)
        (set `self.RobotState` "NewEnumerator0")))))