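; BP_Robot_Seed is a robot pawn that responds to seeding tasks assigned through BP_GameInstance.
; It binds to the task-assigned event on BeginPlay and spawns a BP_Crop at the target for every task received, before checking the robot ID or moving.
; When the ID matches, it uses AI MoveTo to reach the ground-level target, stepping its state enum through travel, a timed wait, and back.
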(event `self.ReceiveBeginPlay`
  (bind _gameinstance (`self.GameInstanceCasting`))
  (add `/Game/Settings/BP_GameInstance.OnTaskAssinged` _gameinstance (delegate `OnTaskRecived`)))

(event `OnTaskRecived`
  (params (TaskData :type "/Game/Datas/Struct/ST_Task Structure"))
  (bind (_taskid _tasktype _assingedrobotid _targetlocation) (break `/Game/Datas/Struct/ST_Task` TaskData))
  (`self.SeedTask` TaskData)
  (if (== _assingedrobotid (`self.RobotId`))
    (set `self.TargetLocation` (`KismetMathLibrary.MakeVector` (.x _targetlocation) (.y _targetlocation)))
    (set `self.RobotState` "NewEnumerator1")
    (`|AIMoveTo` self (`self.TargetLocation`) null
      (:`then`
        (set `self.RobotState` "NewEnumerator2")
        (`KismetSystemLibrary.Delay` 3.0)
        (set `self.RobotState` "NewEnumerator0")))))

(fn `GameInstanceCasting`
  (returns (GameInstance :type "/Game/Settings/BP_GameInstance Object Reference"))
  (bind _asbp_game_instance (cast `/Game/Settings/BP_GameInstance` (`GameplayStatics.GetGameInstance`)))
  (return _asbp_game_instance))

(fn `SeedTask`
  (params (InTaskData :type "/Game/Datas/Struct/ST_Task Structure"))
  (`|SpawnActorFromClass` "/Game/BluePrints/BP_Crop.BP_Crop_C" (`KismetMathLibrary.MakeTransform` InTaskData_TargetLocation_11_9D6EECA142CE8E2E787C0DA5EAE96E88) "Undefined" "MultiplyWithRoot" null null))

(fn `UserConstructionScript`)