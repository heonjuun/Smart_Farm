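; BP_Sencor is a simulated farm environment sensor for one floor, identified by FloorId.
; A looping one-second timer builds an environment struct with random temperature, humidity, soil moisture and CO2, plus fixed LED intensity and a timestamp.
; It passes each reading to BP_GameInstance through CallOnEnviromentUpdated.
; BeginPlay also sets its widget's yaw once, using the dot product of camera forward and widget-to-camera direction.
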(event `self.ReceiveBeginPlay`
  (bind _returnvalue (`GameplayStatics.GetPlayerCameraManager` 0))
  (`KismetSystemLibrary.K2_SetTimer` null "UpdateSencorData" 1.0 true)
  (`SceneComponent.K2_SetWorldRotation` (`self.Widget`) (`KismetMathLibrary.MakeRotator` 0.0 0.0 (`KismetMathLibrary.Dot_VectorVector` (`self.GetActorForwardVector` _returnvalue) (`KismetMathLibrary.Normal` (- (`PlayerCameraManager.GetCameraLocation` _returnvalue) (`SceneComponent.K2_GetComponentLocation` (`self.Widget`)))))) false false))

(fn `UpdateSencorData`
  ; 농장 환경설정
  (bind _asbp_game_instance (cast `/Game/Settings/BP_GameInstance` (`GameplayStatics.GetGameInstance`)))
  (`/Game/Settings/BP_GameInstance.OnEnviromentUpdated` _asbp_game_instance (make `/Game/Datas/Struct/ST_Enviroment` (`KismetMathLibrary.RandomFloatInRange` 18.0 29.0) (`KismetMathLibrary.RandomFloatInRange` 40.0 90.0) (`KismetMathLibrary.RandomFloatInRange` 0.0 1.0) 0.8 (`KismetSystemLibrary.GetGameTimeInSeconds`) (`KismetMathLibrary.RandomFloatInRange` 1100.0 1200.0) (`self.FloorId`))))

(fn `UserConstructionScript`)