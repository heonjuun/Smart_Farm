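; BP_FarmManager is the automated controller of a multi-floor farm, reacting to environment, crop and robot updates broadcast through BP_GameInstance.
; Environment readings drive per-floor cooler, heater, fan and LED commands by threshold, though both fan branches send the same command.
; Crop updates assign watering and harvest tasks to fixed robot IDs.
; Robot updates scan all BP_Robot actors and send low-battery ones to the first charging center found.
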(event `self.ReceiveBeginPlay`
  (add `/Game/Settings/BP_GameInstance.OnEnviromentUpdated` (`self.GameInstanceCasting`) (delegate `OnEnviromentRecived`))
  (add `/Game/Settings/BP_GameInstance.OnCropUpdated` (`self.GameInstanceCasting`) (delegate `On CropRecived`))
  (add `/Game/Settings/BP_GameInstance.OnRobotUpdated` (`self.GameInstanceCasting`) (delegate `OnRobotRecived`)))

(event `OnRobotRecived`
  (params (RobotData :type "/Game/Datas/Struct/ST_Robot Structure"))
  (`self.Battery`))

(event `OnEnviromentRecived`
  (params (EnviromentData :type "/Game/Datas/Struct/ST_Enviroment Structure"))
  ; 온,습도,이산화탄소 농도 조절 센서
  (`|ExecutionSequence`
    (:`then_0`
      (`self.CoolerOn(TemparatureInHot)Off` EnviromentData))
    (:`then_1`
      (`self.HeaterOn(TemparatureInCold)Off` EnviromentData))
    (:`then_2`
      (`self.FanOn(OverCo2)Off` EnviromentData))
    (:`then_3`
      (`self.LedOnOff` EnviromentData))))

(event `On CropRecived`
  (params (CropData :type "/Game/Datas/Struct/ST_Crop Structure"))
  ; 로봇 명령
  (`|ExecutionSequence`
    (:`then_0`
      (`self.WaterTask` CropData))
    (:`then_1`
      (if (`.IsReadyToHarvest_16_9B77FD7C481C21609B170B98946F8210` (break `/Game/Datas/Struct/ST_Crop` CropData))
        (`self.HaverstTask` CropData)))))

(fn `Battery`
  (bind _outactors (`GameplayStatics.GetAllActorsOfClass` "/Game/BluePrints/BP_Robot.BP_Robot_C"))
  (for _array_element _outactors
    (bind _asbp_robot (cast `/Game/BluePrints/BP_Robot` _array_element))
    (if (<= (`self.BatteryLevel`) 20.0)
      (if (not (`|EnumEquality` (`/Game/BluePrints/BP_Robot.RobotState` _asbp_robot) "NewEnumerator3"))
        (bind _outactors_2 (`GameplayStatics.GetAllActorsOfClass` "/Game/BluePrints/BP_BatteryChargingCenter.BP_BatteryChargingCenter_C"))
        (bind _asbp_game_instance (cast `/Game/Settings/BP_GameInstance` (`GameplayStatics.GetGameInstance`)))
        (`/Game/Settings/BP_GameInstance.OnTaskAssinged` _asbp_game_instance (make `/Game/Datas/Struct/ST_Task` 0 "NewEnumerator4" (`/Game/BluePrints/BP_Robot.RobotId` _asbp_robot) (`self.K2_GetActorLocation` (`|GetArrayItem` _outactors_2))))))))

(fn `CoolerOn(TemparatureInHot)Off`
  (params (ST_Enviroment :type "/Game/Datas/Struct/ST_Enviroment Structure (by ref)"))
  (bind (_temparature _humidity _soilmoisture _ledintensity _timestamp _co2level _floorid) (break `/Game/Datas/Struct/ST_Enviroment` ST_Enviroment))
  (bind _gameinstance (`self.GameInstanceCasting`))
  (if (> _temparature (`self.MaxTemparture`))
    (`KismetSystemLibrary.PrintString` "적정온도초과")
    (`/Game/Settings/BP_GameInstance.OnControlCommand` _gameinstance (make `/Game/Datas/Struct/ST_ControlCommand2` 0 "NewEnumerator4" "NewEnumerator0" 0.0 _floorid 0 "적정온도초과입니다."))
    (else
      (`/Game/Settings/BP_GameInstance.OnControlCommand` _gameinstance (make `/Game/Datas/Struct/ST_ControlCommand2` 0 "NewEnumerator4" "NewEnumerator1" 0.0 _floorid 0 "적정온도초과입니다.")))))

(fn `FanOn(OverCo2)Off`
  (params (ST_Enviroment :type "/Game/Datas/Struct/ST_Enviroment Structure (by ref)"))
  (bind (_temparature _humidity _soilmoisture _ledintensity _timestamp _co2level _floorid) (break `/Game/Datas/Struct/ST_Enviroment` ST_Enviroment))
  (bind _gameinstance (`self.GameInstanceCasting`))
  (if (> _co2level (`self.MaxCO2`))
    (`KismetSystemLibrary.PrintString` "CO2초과감지")
    (`/Game/Settings/BP_GameInstance.OnControlCommand` _gameinstance (make `/Game/Datas/Struct/ST_ControlCommand2` 0 "NewEnumerator2" "NewEnumerator0" 0.0 _floorid 0 "CO2농도초과환기를 시작합니다"))
    (else
      (`/Game/Settings/BP_GameInstance.OnControlCommand` _gameinstance (make `/Game/Datas/Struct/ST_ControlCommand2` 0 "NewEnumerator2" "NewEnumerator0" 0.0 _floorid 0 "CO2농도초과환기를 시작합니다")))))

(fn `GameInstanceCasting`
  (returns (GameInstance :type "/Game/Settings/BP_GameInstance Object Reference"))
  (bind _asbp_game_instance (cast `/Game/Settings/BP_GameInstance` (`GameplayStatics.GetGameInstance`)))
  (return _asbp_game_instance))

(fn `HaverstTask`
  (params (ST_Crop :type "/Game/Datas/Struct/ST_Crop Structure (by ref)"))
  (locals (NewLocalVar :type "/Game/Datas/Enum/E_TaskType Enum"))
  (bind (_cropid _floorid _shelfid _growthstage _growthpoint _waterlevel _isreadytoharvest _plantedtime _locationvector) (break `/Game/Datas/Struct/ST_Crop` ST_Crop))
  (if (== true _isreadytoharvest)
    (`/Game/Settings/BP_GameInstance.OnTaskAssinged` (`self.GameInstanceCasting`) (make `/Game/Datas/Struct/ST_Task` 0 "NewEnumerator1" 1 _locationvector _floorid _shelfid "NewEnumerator0" _cropid))))

(fn `HeaterOn(TemparatureInCold)Off`
  (params (ST_Enviroment :type "/Game/Datas/Struct/ST_Enviroment Structure (by ref)"))
  (bind (_temparature _humidity _soilmoisture _ledintensity _timestamp _co2level _floorid) (break `/Game/Datas/Struct/ST_Enviroment` ST_Enviroment))
  (bind _gameinstance (`self.GameInstanceCasting`))
  (if (> (`self.MinTemparature`) _temparature)
    (`KismetSystemLibrary.PrintString` "적정온도감소")
    (`/Game/Settings/BP_GameInstance.OnControlCommand` _gameinstance (make `/Game/Datas/Struct/ST_ControlCommand2` 0 "NewEnumerator3" "NewEnumerator0" 0.0 _floorid 0 "적정온도 아래입니다."))
    (else
      (`/Game/Settings/BP_GameInstance.OnControlCommand` _gameinstance (make `/Game/Datas/Struct/ST_ControlCommand2` 0 "NewEnumerator3" "NewEnumerator1" 0.0 _floorid 0 "적정온도 아래입니다.")))))

(fn `LedOnOff`
  (params (ST_Enviroment :type "/Game/Datas/Struct/ST_Enviroment Structure (by ref)"))
  (bind (_temparature _humidity _soilmoisture _ledintensity _timestamp _co2level _floorid) (break `/Game/Datas/Struct/ST_Enviroment` ST_Enviroment))
  (bind _gameinstance (`self.GameInstanceCasting`))
  (if (<= _ledintensity 0.5)
    (`/Game/Settings/BP_GameInstance.OnControlCommand` _gameinstance (make `/Game/Datas/Struct/ST_ControlCommand2` 0 "NewEnumerator0" "NewEnumerator0" 0.0 _floorid 0 "CO2농도초과환기를 시작합니다"))
    (else
      (`/Game/Settings/BP_GameInstance.OnControlCommand` _gameinstance (make `/Game/Datas/Struct/ST_ControlCommand2` 0 "NewEnumerator0" "NewEnumerator1" 0.0 _floorid 0 "CO2농도초과환기를 시작합니다")))))

(fn `UserConstructionScript`)

(fn `WaterTask`
  (params (ST_Crop :type "/Game/Datas/Struct/ST_Crop Structure (by ref)"))
  (bind (_cropid _floorid _shelfid _growthstage _growthpoint _waterlevel _isreadytoharvest _plantedtime _locationvector) (break `/Game/Datas/Struct/ST_Crop` ST_Crop))
  (if (and (< _growthstage 2) (< _waterlevel 0.3))
    (`/Game/Settings/BP_GameInstance.OnTaskAssinged` (`self.GameInstanceCasting`) (make `/Game/Datas/Struct/ST_Task` 0 "NewEnumerator0" 2 _locationvector _floorid _shelfid "NewEnumerator0" _cropid))))