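; BP_FarmRuntime is the farm manager actor that drives the robot farming loop on a looping timer started at BeginPlay.
; Each UpdateFarm tick has the task scheduler evaluate seed, water and harvest jobs, then the robot manager sends low-battery robots to charge, assigns jobs and updates robot statuses.
; It prints the job queue length for debugging; robot state and type prints are left disconnected.
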(event `self.ReceiveBeginPlay`
  (`KismetSystemLibrary.K2_SetTimer` null "UpdateFarm" (`self.UpdateInterval`) true))

(fn `UpdateFarm`
  (`/Engine/EditorBlueprintResources/StandardMacros.IsValid` (`self.TaskScheudulerRef`)
    (:`Is Valid`
      (`/Game/Farm_Refactor/Managers/BP_TaskScheduler.EvaluateSeedJobs` (`self.TaskScheudulerRef`))
      (`/Game/Farm_Refactor/Managers/BP_TaskScheduler.EvaluateWaterJobs` (`self.TaskScheudulerRef`))
      (`/Game/Farm_Refactor/Managers/BP_TaskScheduler.EvaluateHarvestJobs` (`self.TaskScheudulerRef`))
      (`/Game/Farm_Refactor/Managers/BP_RobotManager.SendLowBatteryRobotsToCharge` (`self.RobotManagerRef`))
      (`/Game/Farm_Refactor/Managers/BP_RobotManager.AssignJobs` (`self.RobotManagerRef`))
      (`/Game/Farm_Refactor/Managers/BP_RobotManager.UpdateRobotStatuses` (`self.RobotManagerRef`))
      (`KismetSystemLibrary.PrintString` (`KismetTextLibrary.Conv_TextToString` (`|FormatText` "잡큐길이:{0}" (`KismetArrayLibrary.Array_Length` (`/Game/Farm_Refactor/Managers/BP_TaskScheduler.JobQueue` (`self.TaskScheudulerRef`))))) true true (struct :`G` 0.66 :`B` 1.0 :`A` 1.0) 22.0))))

(fn `UserConstructionScript`)