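; Farm task scheduler that builds a queue of seed, water and harvest jobs for crop slots, each starting with no assigned robot.
; A looping timer scans the slot manager's registered slots and checks each crop's planted, thirsty and ripe state.
; New jobs take type, priority and work settings from DT_JobDefinition, skipping slots with a matching pending job.
; MarkJobDone updates a job's state in place, leaving it in the queue.
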(event `self.ReceiveBeginPlay`
  (`KismetArrayLibrary.Array_Clear` (`self.JobQueue`))
  (set `self.NextJobID` 1)
  (`KismetSystemLibrary.K2_SetTimer` null "EvaluatePlayJobs" 3.0 true))

(event `EvaluatePlayJobs`
  (`self.EvaluateSeedJobs`)
  (`self.EvaluateWaterJobs`)
  (`self.EvaluateHarvestJobs`))

(fn `AddJob`
  (params (InJob :type "/Game/Farm_Refactor/Data/Struct/ST_FarmJobRow Structure"))
  (`KismetArrayLibrary.Array_Add` (`self.JobQueue`) InJob)
  (`KismetSystemLibrary.PrintString` (`KismetStringLibrary.Concat_StrStr` "job id:" (`KismetStringLibrary.Conv_IntToString` (`.JobId_9_866698BB424272FDC0A30C8C23AD2C4D` (break `/Game/Farm_Refactor/Data/Struct/ST_FarmJobRow` InJob))))))

(fn `EvaluateHarvestJobs`
  (`/Engine/EditorBlueprintResources/StandardMacros.IsValid` (`self.SlotManagerRef`)
    (:`Is Valid`
      (for _array_element (`/Game/Farm_Refactor/Managers/BP_SlotManger.RegisteredSlots` (`self.SlotManagerRef`))
        (bind _cropref (`/Game/Farm_Refactor/Slots/BP_PlantSlot.CropRef` _array_element))
        (`/Engine/EditorBlueprintResources/StandardMacros.IsValid` _cropref
          (:`Is Valid`
            (if (`/Game/Farm_Refactor/Crops/BP_CropBase.bIsPlanted` _cropref)
              (if (`/Game/Farm_Refactor/Crops/BP_CropBase.bReadyToHarvest` _cropref)
                (bind _slotaddress (`/Game/Farm_Refactor/Slots/BP_PlantSlot.SlotAddress` _array_element))
                (bind _found (`self.HasPendingJobForSlot` _slotaddress "NewEnumerator1"))
                (if (not _found)
                  (bind (_outdefinition _found_2) (`self.GetJobDefinition` "NewEnumerator1"))
                  (if _found_2
                    (`self.AddJob` (make `/Game/Farm_Refactor/Data/Struct/ST_FarmJobRow` (`self.NextJobID`) (break `/Game/Farm_Refactor/Data/Struct/ST_JobDefinition` _outdefinition) "NewEnumerator0" -1 _slotaddress (`/Game/Farm_Refactor/Crops/BP_CropBase.CropID` _cropref) (`.Priority_7_05C896434597645046BB3C82781CFE12` (break `/Game/Farm_Refactor/Data/Struct/ST_JobDefinition` _outdefinition)) (`.WorkAmount_9_1B8ADF2B45EC86C2DB0B09B3640AE9D9` (break `/Game/Farm_Refactor/Data/Struct/ST_JobDefinition` _outdefinition)) (`.AcceptanceRadius_12_DDAD4C1C4B14256BF1F01E88A206D5F2` (break `/Game/Farm_Refactor/Data/Struct/ST_JobDefinition` _outdefinition))))
                    (set `self.NextJobID` (+ (`self.NextJobID`) 1))))))))))))

(fn `EvaluateSeedJobs`
  (`/Engine/EditorBlueprintResources/StandardMacros.IsValid` (`self.SlotManagerRef`)
    (:`Is Valid`
      (for _array_element (`/Game/Farm_Refactor/Managers/BP_SlotManger.RegisteredSlots` (`self.SlotManagerRef`))
        (bind _cropref (`/Game/Farm_Refactor/Slots/BP_PlantSlot.CropRef` _array_element))
        (`/Engine/EditorBlueprintResources/StandardMacros.IsValid` _cropref
          (:`Is Valid`
            (if (not (`/Game/Farm_Refactor/Crops/BP_CropBase.bIsPlanted` _cropref))
              (bind _slotaddress (`/Game/Farm_Refactor/Slots/BP_PlantSlot.SlotAddress` _array_element))
              (bind _found (`self.HasPendingJobForSlot` _slotaddress "NewEnumerator2"))
              (if (not _found)
                (bind (_outdefinition _found_2) (`self.GetJobDefinition` "NewEnumerator2"))
                (if _found_2
                  (`self.AddJob` (make `/Game/Farm_Refactor/Data/Struct/ST_FarmJobRow` (`self.NextJobID`) (break `/Game/Farm_Refactor/Data/Struct/ST_JobDefinition` _outdefinition) "NewEnumerator0" -1 _slotaddress (`/Game/Farm_Refactor/Crops/BP_CropBase.CropID` _cropref) (`.Priority_7_05C896434597645046BB3C82781CFE12` (break `/Game/Farm_Refactor/Data/Struct/ST_JobDefinition` _outdefinition)) (`.WorkAmount_9_1B8ADF2B45EC86C2DB0B09B3640AE9D9` (break `/Game/Farm_Refactor/Data/Struct/ST_JobDefinition` _outdefinition)) (`.AcceptanceRadius_12_DDAD4C1C4B14256BF1F01E88A206D5F2` (break `/Game/Farm_Refactor/Data/Struct/ST_JobDefinition` _outdefinition)) (`/Game/Farm_Refactor/Slots/BP_PlantSlot.DefaultCropRowName` _array_element)))
                  (set `self.NextJobID` (+ (`self.NextJobID`) 1)))))))))))

(fn `EvaluateWaterJobs`
  (`/Engine/EditorBlueprintResources/StandardMacros.IsValid` (`self.SlotManagerRef`)
    (:`Is Valid`
      (for _array_element (`/Game/Farm_Refactor/Managers/BP_SlotManger.RegisteredSlots` (`self.SlotManagerRef`))
        (bind _cropref (`/Game/Farm_Refactor/Slots/BP_PlantSlot.CropRef` _array_element))
        (`/Engine/EditorBlueprintResources/StandardMacros.IsValid` _cropref
          (:`Is Valid`
            (if (`/Game/Farm_Refactor/Crops/BP_CropBase.bIsPlanted` _cropref)
              (if (`/Game/Farm_Refactor/Crops/BP_CropBase.bNeedWater` _cropref)
                (bind _slotaddress (`/Game/Farm_Refactor/Slots/BP_PlantSlot.SlotAddress` _array_element))
                (bind _found (`self.HasPendingJobForSlot` _slotaddress))
                (if (not _found)
                  (bind (_outdefinition _found_2) (`self.GetJobDefinition` "NewEnumerator0"))
                  (if _found_2
                    (`self.AddJob` (make `/Game/Farm_Refactor/Data/Struct/ST_FarmJobRow` (`self.NextJobID`) (break `/Game/Farm_Refactor/Data/Struct/ST_JobDefinition` _outdefinition) "NewEnumerator0" -1 _slotaddress (`/Game/Farm_Refactor/Crops/BP_CropBase.CropID` _cropref) (`.Priority_7_05C896434597645046BB3C82781CFE12` (break `/Game/Farm_Refactor/Data/Struct/ST_JobDefinition` _outdefinition)) (`.WorkAmount_9_1B8ADF2B45EC86C2DB0B09B3640AE9D9` (break `/Game/Farm_Refactor/Data/Struct/ST_JobDefinition` _outdefinition)) (`.AcceptanceRadius_12_DDAD4C1C4B14256BF1F01E88A206D5F2` (break `/Game/Farm_Refactor/Data/Struct/ST_JobDefinition` _outdefinition))))
                    (set `self.NextJobID` (+ (`self.NextJobID`) 1))))))))))))

(fn `GetJobDefinition`
  (params (InJobType :type "/Game/Farm_Refactor/Data/Enum/E_JobType Enum" :default "NewEnumerator0"))
  (returns (OutDefinition :type "/Game/Farm_Refactor/Data/Struct/ST_JobDefinition Structure") (Found :type Boolean))
  (locals (LocalRowName :type Name))
  (switch `/Game/Farm_Refactor/Data/Enum/E_JobType` InJobType
    (:`NewEnumerator0`
      (set `local.LocalRowName` "Water"))
    (:`NewEnumerator1`
      (set `local.LocalRowName` "Harvest"))
    (:`NewEnumerator2`
      (set `local.LocalRowName` "Seed")))
  (bind _returnvalue (`|GetDataTableRow` "/Game/Farm_Refactor/Data/DataTable/DT_JobDefinition.DT_JobDefinition" (`local.LocalRowName`))
    (:`then`
      (return _returnvalue true))
    (:`RowNotFound`
      (return (struct) false))))

(fn `HasPendingJobForSlot`
  (params (InAddress :type "/Game/Farm_Refactor/Data/Struct/ST_SlotAddressRow Structure") (InJobType :type "/Game/Farm_Refactor/Data/Enum/E_JobType Enum" :default "NewEnumerator0"))
  (returns (Found :type Boolean))
  (locals (LocalFound :type Boolean))
  (bind (_floorid _shelfid _slotid) (break `/Game/Farm_Refactor/Data/Struct/ST_SlotAddressRow` InAddress))
  (set `local.LocalFound` false)
  (for _array_element (`self.JobQueue`)
    (bind (_jobid _jobtype _jobstate _assingedrobotid _targetaddress) (break `/Game/Farm_Refactor/Data/Struct/ST_FarmJobRow` _array_element))
    (bind (_floorid_2 _shelfid_2 _slotid_2) (break `/Game/Farm_Refactor/Data/Struct/ST_SlotAddressRow` (make `/Game/Farm_Refactor/Data/Struct/ST_SlotAddressRow` (break `/Game/Farm_Refactor/Data/Struct/ST_SlotAddressRow` _targetaddress) (`.ShelfId_7_CFE76FE74A69B24523CBFCBC9EAE4B9B` (break `/Game/Farm_Refactor/Data/Struct/ST_SlotAddressRow` _targetaddress)) (`.SlotId_8_6BA64B8643A4E049FB8BD399DC3C3F01` (break `/Game/Farm_Refactor/Data/Struct/ST_SlotAddressRow` _targetaddress)))))
    (if (and (`|EnumEquality` _jobtype InJobType) (== _floorid _floorid_2) (== _shelfid _shelfid_2) (== _slotid _slotid_2) (or (`|EnumEquality` _jobstate "NewEnumerator0") (`|EnumEquality` _jobstate "NewEnumerator1")))
      (set `local.LocalFound` true)
      (break)))
  (return (`local.LocalFound`)))

(fn `MarkJobDone`
  (params (InJobID :type Integer))
  (for (_array_element _array_index) (`self.JobQueue`)
    (bind (_jobid _jobtype _jobstate _assingedrobotid _targetaddress _targetcropid _priority) (break `/Game/Farm_Refactor/Data/Struct/ST_FarmJobRow` _array_element))
    (if (== InJobID _jobid)
      (`KismetArrayLibrary.Array_Set` (`self.JobQueue`) _array_index (make `/Game/Farm_Refactor/Data/Struct/ST_FarmJobRow` _jobid _jobtype "NewEnumerator3" _assingedrobotid _targetaddress _targetcropid _priority))
      (`KismetSystemLibrary.PrintString` "MarkJobDone")
      (`KismetSystemLibrary.PrintString` (`KismetStringLibrary.Concat_StrStr` "jobdone job id:" (`KismetStringLibrary.Conv_IntToString` _jobid)))
      (break))))

(fn `UserConstructionScript`)