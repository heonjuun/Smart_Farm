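; BP_SlotManger is a farm manager that keeps a registry of the plant slots in the level.
; On BeginPlay it gathers every BP_PlantSlot and gives each an address from the default floor and shelf plus an incrementing slot ID.
; GetSlotByAddress searches the registry linearly for a matching floor, shelf and slot.
; RegisterSlot adds a single slot without duplicates but assigns it no address.
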(event `self.ReceiveBeginPlay`
  (`self.RegisterAllSlots`))

(fn `GetSlotByAddress`
  (params (InAddress :type "/Game/Farm_Refactor/Data/Struct/ST_SlotAddressRow Structure"))
  (returns (FoundSlot :type "/Game/Farm_Refactor/Slots/BP_PlantSlot Object Reference") (bFound :type Boolean))
  (locals (LocalFoundSlot :type "/Game/Farm_Refactor/Slots/BP_PlantSlot Object Reference") (LocalFound :type Boolean))
  (for _array_element (`self.RegisteredSlots`)
    (bind (_floorid _shelfid _slotid) (break `/Game/Farm_Refactor/Data/Struct/ST_SlotAddressRow` (`/Game/Farm_Refactor/Slots/BP_PlantSlot.SlotAddress` _array_element)))
    (if (and (== InAddress_FloorId_6_2B87F1824A92988B91E9BD8CD431B6AA _floorid) (== InAddress_ShelfId_7_CFE76FE74A69B24523CBFCBC9EAE4B9B _shelfid) (== InAddress_SlotId_8_6BA64B8643A4E049FB8BD399DC3C3F01 _slotid))
      (set `local.LocalFoundSlot` _array_element)
      (set `local.LocalFound` true)
      (break)))
  (return (`local.LocalFoundSlot`) (`local.LocalFound`)))

(fn `RegisterAllSlots`
  (`KismetArrayLibrary.Array_Clear` (`self.RegisteredSlots`))
  (set `self. NextSlotID` 1)
  (bind _outactors (`GameplayStatics.GetAllActorsOfClass` "/Game/Farm_Refactor/Slots/BP_PlantSlot.BP_PlantSlot_C"))
  (for _array_element _outactors
    (bind _asbp_plant_slot (cast `/Game/Farm_Refactor/Slots/BP_PlantSlot` _array_element))
    (`KismetArrayLibrary.Array_Add` (`self.RegisteredSlots`) _asbp_plant_slot)
    (set `/Game/Farm_Refactor/Slots/BP_PlantSlot.SlotAddress` (make `/Game/Farm_Refactor/Data/Struct/ST_SlotAddressRow` (`self.DefaultFloorId`) (`self.DefaultShelfId`) (`self. NextSlotID`)) _asbp_plant_slot)
    (set `self. NextSlotID` (+ (`self. NextSlotID`) 1))))

(fn `RegisterSlot`
  (params (InSlot :type "/Game/Farm_Refactor/Slots/BP_PlantSlot Object Reference"))
  (`/Engine/EditorBlueprintResources/StandardMacros.IsValid` InSlot
    (:`Is Valid`
      (if (not (`KismetArrayLibrary.Array_Contains` (`self.RegisteredSlots`) InSlot))
        (`KismetArrayLibrary.Array_Add` (`self.RegisteredSlots`) InSlot)
        (`KismetSystemLibrary.PrintString` "slot registerd")))))

(fn `UserConstructionScript`)