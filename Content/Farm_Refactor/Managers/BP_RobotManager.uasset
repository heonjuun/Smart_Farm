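; Farm robot manager that keeps a registry of robots and dispatches work and charging commands to them; its functions are called externally.
; AssignJobs gives each idle, work-capable robot the highest-priority matching job from the TaskScheduler's queue, then writes that job entry back.
; SendLowBatteryRobotsToCharge sends a different command type to idle robots that cannot work.
; UpdateRobotStatuses rebuilds the status list, and ResolveHarvestStorage caches the harvest storage actor.
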(fn `AssignJobs`
  (locals (BestJob :type "/Game/Farm_Refactor/Data/Struct/ST_FarmJobRow Structure" :default (struct :`JobType` "NewEnumerator0" :`JobState` "NewEnumerator0" :`TargetAddress` (struct))) (BestJobIndex :type Integer) (BestPriority :type Integer))
  (bind (_bestjob_jobid _bestjob_jobtype) (break `/Game/Farm_Refactor/Data/Struct/ST_FarmJobRow` (`local.BestJob`)))
  (`/Engine/EditorBlueprintResources/StandardMacros.IsValid` (`self.TaskSchedulerRef`)
    (:`Is Valid`
      (for (_array_element _array_index) (`self.RegisteredRobots`)
        (bind _canwork (`/Game/Farm_Refactor/Robots/BP_RobotBase.CanWork` _array_element))
        (if (and _canwork (`|EnumEquality` (`/Game/Farm_Refactor/Robots/BP_RobotBase.RobotState` _array_element) "NewEnumerator0") (not (`/Game/Farm_Refactor/Robots/BP_RobotBase.bHasJob` _array_element)))
          (set `local.BestJobIndex` -1)
          (set `local.BestPriority` -1)
          (for (_array_element_2 _array_index_2) (`/Game/Farm_Refactor/Managers/BP_TaskScheduler.JobQueue` (`self.TaskSchedulerRef`))
            (bind (_jobid _jobtype _jobstate _assingedrobotid _targetaddress _targetcropid _priority) (break `/Game/Farm_Refactor/Data/Struct/ST_FarmJobRow` _array_element_2))
            (bind _cando (`/Game/Farm_Refactor/Robots/BP_RobotBase.CanDoJobType` _array_element _jobtype))
            (if (and _cando (`|EnumEquality` _jobstate "NewEnumerator0") (> _priority (`local.BestPriority`)))
              (set `local.BestJob` _array_element_2)
              (set `local.BestJobIndex` _array_index_2)
              (set `local.BestPriority` _priority)))
          (if (!= (`local.BestJobIndex`) -1)
            (`/Game/Farm_Refactor/Robots/BP_RobotBase.ReciveControlCommand` _array_element (make `/Game/Farm_Refactor/Data/Struct/ST_controlCommand` (`self.NextCommandId`) "NewEnumerator0" _array_index (`local.BestJob`)))
            (bind _structout (setmembers `/Game/Farm_Refactor/Data/Struct/ST_FarmJobRow` :`StructRef` (`local.BestJob`)))
            (`KismetArrayLibrary.Array_Set` (`/Game/Farm_Refactor/Managers/BP_TaskScheduler.JobQueue` (`self.TaskSchedulerRef`)) (`local.BestJobIndex`) _structout)
            (`KismetSystemLibrary.PrintString` (`KismetTextLibrary.Conv_TextToString` (`|FormatText` "best job index:{0}" (`local.BestJobIndex`))) true true (struct :`G` 0.66 :`B` 1.0 :`A` 1.0) 22.0)
            (`KismetSystemLibrary.PrintString` (`KismetTextLibrary.Conv_TextToString` (`|FormatText` "robot type:{0}" (`|GetEnumeratorNameAsString` _bestjob_jobtype))) true true (struct :`G` 0.66 :`B` 1.0 :`A` 1.0) 22.0)))))))

(fn `RegisterRobot`
  (params (InRobot :type "/Game/Farm_Refactor/Robots/BP_RobotBase Object Reference"))
  ; 로봇 등록 함수(레지스터로봇함수가 값을 받아서 값이 존재하면 포함되지않으면 등록)
  (`/Engine/EditorBlueprintResources/StandardMacros.IsValid` InRobot
    (:`Is Valid`
      (if (not (`KismetArrayLibrary.Array_Contains` (`self.RegisteredRobots`) InRobot))
        (`KismetArrayLibrary.Array_Add` (`self.RegisteredRobots`) InRobot)))))

(fn `ResolveHarvestStorage`
  (bind _returnvalue (`GameplayStatics.GetActorOfClass` "/Game/Farm_Refactor/HarvestStorage/BP_HarvestStorage.BP_HarvestStorage_C"))
  (bind _asbp_harvest_storage (cast `/Game/Farm_Refactor/HarvestStorage/BP_HarvestStorage` _returnvalue))
  (set `self.HaverstStorageRef` _asbp_harvest_storage)
  (`KismetSystemLibrary.PrintString` "robotmanager stroage found" true true (struct :`G` 0.66 :`B` 1.0 :`A` 1.0) 22.0))

(fn `SendLowBatteryRobotsToCharge`
  (for _array_element (`self.RegisteredRobots`)
    (`/Engine/EditorBlueprintResources/StandardMacros.IsValid` _array_element
      (:`Is Valid`
        (bind _canwork (`/Game/Farm_Refactor/Robots/BP_RobotBase.CanWork` _array_element))
        (if (and (not _canwork) (`|EnumEquality` (`/Game/Farm_Refactor/Robots/BP_RobotBase.RobotState` _array_element) "NewEnumerator0") (not (`/Game/Farm_Refactor/Robots/BP_RobotBase.bHasJob` _array_element)) (not (`/Game/Farm_Refactor/Robots/BP_RobotBase.bIsCharging` _array_element)))
          (`/Game/Farm_Refactor/Robots/BP_RobotBase.ReciveControlCommand` _array_element (make `/Game/Farm_Refactor/Data/Struct/ST_controlCommand` (`self.NextCommandId`) "NewEnumerator3" (`/Game/Farm_Refactor/Robots/BP_RobotBase.RobotID` _array_element) (struct :`JobType` "NewEnumerator0" :`JobState` "NewEnumerator0" :`TargetAddress` (struct) :`CropRowName` "False")))
          (set `self.NextCommandId` (+ (`self.NextCommandId`) 1)))))))

(fn `UpdateRobotStatuses`
  (`KismetArrayLibrary.Array_Clear` (`self.RobotStatuses`))
  (for _array_element (`self.RegisteredRobots`)
    (`/Engine/EditorBlueprintResources/StandardMacros.IsValid` _array_element
      (:`Is Valid`
        (bind _robotstatus (`/Game/Farm_Refactor/Robots/BP_RobotBase.MakeRobotStatus` _array_element))
        (`KismetArrayLibrary.Array_Add` (`self.RobotStatuses`) _robotstatus)))))

(fn `UserConstructionScript`)