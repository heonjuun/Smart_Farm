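; Base farm robot character that performs water, seed and harvest jobs on crop slots.
; It loads stats from a data table, registers with the robot manager and accepts commands.
; Jobs and charge or storage trips are passed to BP_RobotAI through blackboard keys.
; Finished jobs drain battery and notify the task scheduler; a looping timer refreshes the diagnostic widget.
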(event `StartMoveCurrentJob`
  (bind _slotmanagerref (`self.SlotManagerRef`))
  (bind (_currentjob_jobid _currentjob_jobtype _currentjob_jobstate _currentjob_assingedrobotid _currentjob_targetaddress _currentjob_targetcropid _currentjob_priority _currentjob_workamount _currentjob_acceptanceradius) (break `/Game/Farm_Refactor/Data/Struct/ST_FarmJobRow` (`self.CurrentJob`)))
  (bind (_currentjob_jobid_2 _currentjob_jobtype_2 _currentjob_jobstate_2 _currentjob_assingedrobotid_2 _currentjob_targetaddress_2) (break `/Game/Farm_Refactor/Data/Struct/ST_FarmJobRow` (`self.CurrentJob`)))
  (set `self.RobotState` "NewEnumerator5")
  (`KismetSystemLibrary.PrintString` "RobotState:Moving")
  (`/Engine/EditorBlueprintResources/StandardMacros.IsValid` _slotmanagerref
    (:`Is Valid`
      (bind (_foundslot _bfound) (`/Game/Farm_Refactor/Managers/BP_SlotManger.GetSlotByAddress` _slotmanagerref _currentjob_targetaddress_2))
      (if _bfound
        (`/Engine/EditorBlueprintResources/StandardMacros.IsValid` _foundslot
          (:`Is Valid`
            (set `self.MoveTargetSlot` _foundslot)
            (set `self.CurrentTargetLocation` (`SceneComponent.K2_GetComponentLocation` (`/Game/Farm_Refactor/Slots/BP_PlantSlot.WorkPoint` _foundslot)))
            (`|AIMoveTo` self (`self.CurrentTargetLocation`) null _currentjob_acceptanceradius true
              (:`then`
                (`KismetSystemLibrary.PrintString` "Move Requested" true true (struct :`G` 0.66 :`B` 1.0 :`A` 1.0) 0.2))
              (:`OnSuccess`
                (set `self.RobotState` "NewEnumerator2")
                (`self.ExecuteCurrentJob`))
              (:`OnFail`
                (`KismetSystemLibrary.PrintString` "failed")))))))))

(event `self.ReceiveBeginPlay`
  (bind _returnvalue (`GameplayStatics.GetActorOfClass` "/Game/Farm_Refactor/Managers/BP_RobotManager.BP_RobotManager_C"))
  (bind _asbp_robot_manager (cast `/Game/Farm_Refactor/Managers/BP_RobotManager` _returnvalue))
  (`self.LoadRobotDefinition`)
  (`/Game/Farm_Refactor/Managers/BP_RobotManager.RegisterRobot` _asbp_robot_manager self)
  (`self.UpdateRobotDiagnosticUI`)
  (`KismetSystemLibrary.K2_SetTimer` null "UpdateRobotDiagnosticUI" 0.2 true))

(event `StartCharging`
  (bind _returnvalue (`KismetSystemLibrary.K2_SetTimerDelegate` (delegate `ChargeTick`) 0.2 true))
  (set `self.ChargingTimer` _returnvalue))

(event `ChargeTick`
  (set `self.BatteryLevel` (`KismetMathLibrary.FClamp` (+ (`self.BatteryLevel`) (`self.ChargeRate`)) 0.0 (`self.BatteryMax`)))
  (`KismetSystemLibrary.PrintString` (`KismetStringLibrary.Concat_StrStr` "Battery:" (`KismetStringLibrary.Conv_DoubleToString` (`self.BatteryLevel`))))
  (if (>= (`self.BatteryLevel`) (`self.BatteryMax`))
    (`KismetSystemLibrary.K2_ClearAndInvalidateTimerHandle` (`self.ChargingTimer`))
    (set `self.bIsCharging` false)
    (set `self.RobotState` "NewEnumerator0")))

(fn `AssignJob`
  (params (InJob :type "/Game/Farm_Refactor/Data/Struct/ST_FarmJobRow Structure"))
  (bind _slotmanagerref (`self.SlotManagerRef`))
  (bind (_currentjob_jobid _currentjob_jobtype _currentjob_jobstate _currentjob_assingedrobotid _currentjob_targetaddress) (break `/Game/Farm_Refactor/Data/Struct/ST_FarmJobRow` (`self.CurrentJob`)))
  (bind (_currentjob_jobid_2 _currentjob_jobtype_2) (break `/Game/Farm_Refactor/Data/Struct/ST_FarmJobRow` (`self.CurrentJob`)))
  (set `self.CurrentJob` InJob)
  (set `self.bHasJob` true)
  (set `self.RobotState` "NewEnumerator1")
  (`/Engine/EditorBlueprintResources/StandardMacros.IsValid` _slotmanagerref
    (:`Is Valid`
      (switch `/Game/Farm_Refactor/Data/Enum/E_JobType` _currentjob_jobtype
        (:`NewEnumerator0`
          (set `self.LogReference` "Water"))
        (:`NewEnumerator1`
          (set `self.LogReference` "Harvest"))
        (:`NewEnumerator2`
          (set `self.LogReference` "Seed")))
      (bind (_foundslot _bfound) (`/Game/Farm_Refactor/Managers/BP_SlotManger.GetSlotByAddress` _slotmanagerref _currentjob_targetaddress))
      (if _bfound
        (bind _asbp_robot_ai (cast `/Game/Farm_Refactor/Robots/BP_RobotAI` (`self.GetController`)))
        (set `self.MoveTargetSlot` _foundslot)
        (set `self.CurrentTargetLocation` (`SceneComponent.K2_GetComponentLocation` (`/Game/Farm_Refactor/Slots/BP_PlantSlot.WorkPoint` _foundslot)))
        (bind _returnvalue (`AIBlueprintHelperLibrary.GetBlackboard` _asbp_robot_ai))
        (`BlackboardComponent.SetValueAsBool` _returnvalue "HasJob" true)
        (`BlackboardComponent.SetValueAsVector` _returnvalue "CurrentTargetLocation" (`self.CurrentTargetLocation`))
        (`BlackboardComponent.SetValueAsEnum` _returnvalue "JobType" _currentjob_jobtype_2)))))

(fn `CanDoJobType`
  (params (InJobType :type "/Game/Farm_Refactor/Data/Enum/E_JobType Enum" :default "NewEnumerator0"))
  (returns (CanDo :type Boolean))
  (switch `/Game/Farm_Refactor/Data/Enum/E_JobType` InJobType
    (:`NewEnumerator0`
      (return (`self.CanWater`)))
    (:`NewEnumerator1`
      (return (`self.CanHarvest`)))
    (:`NewEnumerator2`
      (return (`self.CanSeed`)))))

(fn `CanWork`
  (returns (CanWork :type Boolean))
  (return (>= (`self.BatteryLevel`) (`self.MinBatteryToWork`))))

(fn `CompleteCurrentJob`
  (bind _currentjob_jobid (break `/Game/Farm_Refactor/Data/Struct/ST_FarmJobRow` (`self.CurrentJob`)))
  (`/Engine/EditorBlueprintResources/StandardMacros.IsValid` (`self.TaskSchedulerRef`)
    (:`Is Valid`
      (set `self.CompleteJobType` (`.JobType_10_33CECBB948B6C42587019693E1464A87` (break `/Game/Farm_Refactor/Data/Struct/ST_FarmJobRow` (`self.CurrentJob`))))
      (`/Game/Farm_Refactor/Managers/BP_TaskScheduler.MarkJobDone` (`self.TaskSchedulerRef`) _currentjob_jobid)
      (set `self.RobotState` "NewEnumerator6")
      (set `self.bHasJob` false)
      (set `self.CurrentJob` (make `/Game/Farm_Refactor/Data/Struct/ST_FarmJobRow` -1 "NewEnumerator0" "NewEnumerator5" -1))
      (set `self.MoveTargetSlot` null)
      (set `self.CurrentTargetLocation` (0.0 0.0 0.0))
      (set `self.RobotState` "NewEnumerator0")
      (cast `/Game/Farm_Refactor/Robots/BP_RobotAI` (`self.GetController`))
      (`BlackboardComponent.SetValueAsBool` (`AIBlueprintHelperLibrary.GetBlackboard` null) "HasJob" false)
      (`BlackboardComponent.SetValueAsBool` (`AIBlueprintHelperLibrary.GetBlackboard` null) "ShouldCharge" false)
      (bind _canwork (`self.CanWork`))
      (if _canwork
        (switch `/Game/Farm_Refactor/Data/Enum/E_JobType` (`self.CompleteJobType`)
          (:`NewEnumerator0`
            (set `self.RobotState` "NewEnumerator0"))
          (:`NewEnumerator1`
            (`self.PrePareReturnToStorageByBlackTree`))
          (:`NewEnumerator2`
            (set `self.RobotState` "NewEnumerator0")))
        (else
          (`self.PrePareChargeByBlackTree`))))))

(fn `ConSumeBattery`
  (params (Amount :type "Float (double-precision)"))
  (set `self.BatteryLevel` (`KismetMathLibrary.FClamp` (- (`self.BatteryLevel`) Amount) 0.0 (`self.BatteryMax`))))

(fn `DeliverHarvestToStorage`
  (bind _harveststorageref (`self.HarvestStorageRef`))
  (if (> (`self.PendingHarverstAmount`) 0)
    (`/Engine/EditorBlueprintResources/StandardMacros.IsValid` _harveststorageref
      (:`Is Valid`
        (`/Game/Farm_Refactor/HarvestStorage/BP_HarvestStorage.AddHarvestItem` _harveststorageref (`self.PendingHarverstCropName`) (`self.PendingHarverstAmount`))
        (set `self.PendingHarverstAmount` 0)
        (set `self.PendingHarverstCropName` "None")))))

(fn `ExecuteCurrentJob`
  (bind (_currentjob_jobid _currentjob_jobtype) (break `/Game/Farm_Refactor/Data/Struct/ST_FarmJobRow` (`self.CurrentJob`)))
  (if (`|EnumEquality` _currentjob_jobtype "NewEnumerator0")
    (`self.ExecuteWaterJob`)
    (elif (`|EnumEquality` _currentjob_jobtype "NewEnumerator1")
      (`self.ExecuteHarvestJobs`)
      (elif (`|EnumEquality` _currentjob_jobtype "NewEnumerator2")
        (`self.ExecuteSeedJobs`)))))

(fn `ExecuteHarvestJobs`
  (bind _movetargetslot (`self.MoveTargetSlot`))
  (bind _cropref (`/Game/Farm_Refactor/Slots/BP_PlantSlot.CropRef` _movetargetslot))
  (`/Engine/EditorBlueprintResources/StandardMacros.IsValid` _movetargetslot
    (:`Is Valid`
      (`/Engine/EditorBlueprintResources/StandardMacros.IsValid` _cropref
        (:`Is Valid`
          (set `self.PendingHarverstCropName` (`/Game/Farm_Refactor/Crops/BP_CropBase.CurrentCropRowName` _cropref))
          (`/Game/Farm_Refactor/Crops/BP_CropBase.HarvestCrop` _cropref)
          (set `self.PendingHarverstAmount` (+ (`self.PendingHarverstAmount`) 1))
          (`self.ConSumeBattery` (`self.BatteryCostPerJob`))
          (`self.CompleteCurrentJob`))))))

(fn `ExecuteSeedJobs`
  (bind (_currentjob_jobid _currentjob_jobtype _currentjob_jobstate _currentjob_assingedrobotid _currentjob_targetaddress _currentjob_targetcropid _currentjob_priority _currentjob_workamount _currentjob_acceptanceradius _currentjob_croprowname) (break `/Game/Farm_Refactor/Data/Struct/ST_FarmJobRow` (`self.CurrentJob`)))
  (bind _movetargetslot (`self.MoveTargetSlot`))
  (`/Engine/EditorBlueprintResources/StandardMacros.IsValid` _movetargetslot
    (:`Is Valid`
      (`/Game/Farm_Refactor/Slots/BP_PlantSlot.SpawnCrop` _movetargetslot _currentjob_croprowname)
      (`self.ConSumeBattery` (`self.BatteryCostPerJob`))
      (`self.CompleteCurrentJob`))))

(fn `ExecuteWaterJob`
  (bind (_currentjob_jobid _currentjob_jobtype _currentjob_jobstate _currentjob_assingedrobotid _currentjob_targetaddress _currentjob_targetcropid _currentjob_priority _currentjob_workamount) (break `/Game/Farm_Refactor/Data/Struct/ST_FarmJobRow` (`self.CurrentJob`)))
  (bind _movetargetslot (`self.MoveTargetSlot`))
  (bind _cropref (`/Game/Farm_Refactor/Slots/BP_PlantSlot.CropRef` _movetargetslot))
  (`/Engine/EditorBlueprintResources/StandardMacros.IsValid` _movetargetslot
    (:`Is Valid`
      (`/Engine/EditorBlueprintResources/StandardMacros.IsValid` _cropref
        (:`Is Valid`
          (`/Game/Farm_Refactor/Crops/BP_CropBase.ApplyWater` _cropref _currentjob_workamount)
          (`self.ConSumeBattery` (`self.BatteryCostPerJob`))
          (`self.CompleteCurrentJob`))))))

(fn `GetRobotLogMessage`
  (returns (OutMessage :type Text) (OutColor :type "LinearColor Structure"))
  (bind _returnvalue (`|GetDataTableRow` "/Game/Farm_Refactor/Data/DataTable/DT_RobotLog.DT_RobotLog" (`self.LogReference`))
    (:`then`
      (return (break `/Game/Farm_Refactor/Data/Struct/ST_RobotLog` _returnvalue) (`.Log_Color_7_B40EEC5F486E5D75D068FC9251C77819` (break `/Game/Farm_Refactor/Data/Struct/ST_RobotLog` _returnvalue))))
    (:`RowNotFound`
      (return "UnKnown" (struct :`A` 1.0)))))

(fn `LoadRobotDefinition`
  (bind _returnvalue (`|GetDataTableRow` "/Game/Farm_Refactor/Data/DataTable/DT_RobotDefinition.DT_RobotDefinition" (`self.RobotDefinitionRowName`))
    (:`then`
      (set `self.RobotType` (break `/Game/Farm_Refactor/Data/Struct/ST_RobotDefinition` _returnvalue))
      (set `self.CanWater` (`.CanWater_9_CB0D803547EA8D9A4F25D79001AC78C2` (break `/Game/Farm_Refactor/Data/Struct/ST_RobotDefinition` _returnvalue)))
      (set `self.CanHarvest` (`.CanHaverst_10_B57E991B4D22423CE1A8F293A39DB1A2` (break `/Game/Farm_Refactor/Data/Struct/ST_RobotDefinition` _returnvalue)))
      (set `self.CanSeed` (`.CanSeed_13_5E715C3346A90A9C4E5AFB9589529C0E` (break `/Game/Farm_Refactor/Data/Struct/ST_RobotDefinition` _returnvalue)))
      (set `self.MoveSpeed` (`.MoveSpeed_15_2DC1EB5E405AFC13EA017C9B727ED5B2` (break `/Game/Farm_Refactor/Data/Struct/ST_RobotDefinition` _returnvalue)))
      (set `self.BatteryMax` (`.BatteryMax_20_570F4CEC494B6245D957EFA445BD179D` (break `/Game/Farm_Refactor/Data/Struct/ST_RobotDefinition` _returnvalue)))
      (set `self.BatteryLevel` (`self.BatteryMax`))
      (set `CharacterMovementComponent.MaxWalkSpeed` (`.MoveSpeed_15_2DC1EB5E405AFC13EA017C9B727ED5B2` (break `/Game/Farm_Refactor/Data/Struct/ST_RobotDefinition` _returnvalue)) (`self.CharacterMovement`)))))

(fn `MakeRobotStatus`
  (returns (RobotStatus :type "/Game/Farm_Refactor/Data/Struct/ST_RobotStatus Structure"))
  (bind (_currentjob_jobid _currentjob_jobtype) (break `/Game/Farm_Refactor/Data/Struct/ST_FarmJobRow` (`self.CurrentJob`)))
  (return (make `/Game/Farm_Refactor/Data/Struct/ST_RobotStatus` (`self.RobotID`) (`self.RobotState`) _currentjob_jobid _currentjob_jobtype (`self.K2_GetActorLocation`) (`self.bHasJob`) (`self.BatteryLevel`))))

(fn `PrePareChargeByBlackTree`
  (`/Engine/EditorBlueprintResources/StandardMacros.IsValid` (`self.ChargingStationRef`)
    (:`Is Valid`
      (set `self.CurrentTargetLocation` (`SceneComponent.K2_GetComponentLocation` (`/Game/Farm_Refactor/ChargingStation/BP_ChargingStation.ChargePoint` (`self.ChargingStationRef`))))
      (set `self.RobotState` "NewEnumerator5")
      (set `self.bHasJob` false)
      (`BlackboardComponent.SetValueAsBool` (`AIBlueprintHelperLibrary.GetBlackboard` null) "HasJob" false)
      (`BlackboardComponent.SetValueAsVector` (`AIBlueprintHelperLibrary.GetBlackboard` null) "ChargeLocation" (`SceneComponent.K2_GetComponentLocation` (`/Game/Farm_Refactor/ChargingStation/BP_ChargingStation.ChargePoint` (`self.ChargingStationRef`))))
      (`BlackboardComponent.SetValueAsBool` (`AIBlueprintHelperLibrary.GetBlackboard` null) "ShouldCharge" true))))

(fn `PrePareReturnToStorageByBlackTree`
  (bind _returnvalue (`AIBlueprintHelperLibrary.GetBlackboard` null))
  (bind _harveststorageref (`self.HarvestStorageRef`))
  (`/Engine/EditorBlueprintResources/StandardMacros.IsValid` _harveststorageref
    (:`Is Valid`
      (`BlackboardComponent.SetValueAsVector` _returnvalue "StandByLocation" (`SceneComponent.K2_GetComponentLocation` (`/Game/Farm_Refactor/HarvestStorage/BP_HarvestStorage.StandByPoint` _harveststorageref)))
      (`BlackboardComponent.SetValueAsBool` _returnvalue "ShouldReturnToStandBy" true)
      (set `self.RobotState` "NewEnumerator5"))))

(fn `ReciveControlCommand`
  (params (InCommand :type "/Game/Farm_Refactor/Data/Struct/ST_controlCommand Structure"))
  (bind (_commandid _commandtype _targetrobotid _jobdata) (break `/Game/Farm_Refactor/Data/Struct/ST_controlCommand` InCommand))
  (if true
    (switch `/Game/Farm_Refactor/Data/Enum/E_ControlCommandType` _commandtype
      (:`NewEnumerator0`
        (`self.AssignJob` _jobdata))
      (:`NewEnumerator3`
        (`self.PrePareChargeByBlackTree`)))))

(fn `UpdateRobotDiagnosticUI`
  (locals (NewLocalVar :type "/Game/Farm_Refactor/Data/Enum/E_JobState Enum"))
  (bind (_jobid _jobtype _jobstate _assingedrobotid) (break `/Game/Farm_Refactor/Data/Struct/ST_FarmJobRow` (`self.CurrentJob`)))
  (bind _aswbp_robot_diagnostic (cast `/Game/Farm_Refactor/UI/WBP_RobotDiagnostic` (`WidgetComponent.GetUserWidgetObject` (`self.RobotDiagnosticwidget`))))
  (`TextBlock.SetText` (`/Game/Farm_Refactor/UI/WBP_RobotDiagnostic.Txt_RobotID` _aswbp_robot_diagnostic) (`|FormatText` "RobotID:{id}" _assingedrobotid))
  (`TextBlock.SetText` (`/Game/Farm_Refactor/UI/WBP_RobotDiagnostic.Txt_State` _aswbp_robot_diagnostic) (`|FormatText` "State:{state}" (`|GetEnumeratorNameAsString` _jobstate)))
  (if (and (!= _jobid -1) (`self.bHasJob`))
    (bind _txt_job (`/Game/Farm_Refactor/UI/WBP_RobotDiagnostic.Txt_Job` _aswbp_robot_diagnostic))
    (`TextBlock.SetText` _txt_job (`|FormatText` "Job:{job}" (`|GetEnumeratorNameAsString` _jobtype)))
    (else
      (`TextBlock.SetText` _txt_job (`|FormatText` "Job:None"))))
  (`TextBlock.SetText` (`/Game/Farm_Refactor/UI/WBP_RobotDiagnostic.Txt_Battery` _aswbp_robot_diagnostic) (`|FormatText` "Battery:{battery}/{max}" (`self.BatteryLevel`) (`self.BatteryMax`)))
  (`ProgressBar.SetPercent` (`/Game/Farm_Refactor/UI/WBP_RobotDiagnostic.PB_Battery` _aswbp_robot_diagnostic) (`KismetMathLibrary.FClamp` (/ (`self.BatteryLevel`) (`self.BatteryMax`))))
  (bind _outmessage (`self.GetRobotLogMessage`))
  (`TextBlock.SetText` (`/Game/Farm_Refactor/UI/WBP_RobotDiagnostic.Txt_Log` _aswbp_robot_diagnostic) _outmessage))

(fn `UserConstructionScript`)