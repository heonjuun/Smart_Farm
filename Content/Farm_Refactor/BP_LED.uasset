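; BP_LED is a farm LED light that switches on or off in response to control commands for its floor.
; On BeginPlay it binds to the OnControlCommand event on BP_GameInstance.
; Commands matching its device type and FloorId set LedLight to the IntenCity intensity for the first command type, or to zero otherwise.
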(event `self.ReceiveBeginPlay`
  (bind _newparam (`self.GameInstanceCasting`))
  (add `/Game/Settings/BP_GameInstance.OnControlCommand` _newparam (delegate `OnControlCommandRecieve`)))

(event `OnControlCommandRecieve`
  (params (ControlCommand :type "/Game/Datas/Struct/ST_ControlCommand2 Structure"))
  (bind (_command_id _targetdevice _commandtype _ledvalue _floorid) (break `/Game/Datas/Struct/ST_ControlCommand2` ControlCommand))
  (if (`|EnumEquality` _targetdevice "NewEnumerator0")
    (if (== _floorid (`self.FloorId`))
      (if (`|EnumEquality` _commandtype "NewEnumerator0")
        (`LightComponent.SetIntensity` (`self.LedLight`) (`self.IntenCity`))
        (else
          (`LightComponent.SetIntensity` (`self.LedLight`) 0.0))))))

(fn `GameInstanceCasting`
  (returns (NewParam :type "/Game/Settings/BP_GameInstance Object Reference"))
  (bind _asbp_game_instance (cast `/Game/Settings/BP_GameInstance` (`GameplayStatics.GetGameInstance`)))
  (return _asbp_game_instance))

(fn `UserConstructionScript`)