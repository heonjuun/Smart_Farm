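; BP_FarmRuntime is a farm manager actor that periodically drives the farm's task scheduler.
; On BeginPlay it starts a looping timer at UpdateInterval that calls UpdateFarm.
; UpdateFarm tells the referenced scheduler, when valid, to evaluate water jobs, then prints its job queue length as debug output.
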(event `self.ReceiveBeginPlay`
  (`KismetSystemLibrary.K2_SetTimer` null "UpdateFarm" (`self.UpdateInterval`) true))

(fn `UpdateFarm`
  (bind _taskscheudulerref (`self.TaskScheudulerRef`))
  (`/Engine/EditorBlueprintResources/StandardMacros.IsValid` _taskscheudulerref
    (:`Is Valid`
      (`/Game/Farm_Refactor/Mangers/BP_TaskScheduler.EvaluateWaterJobs` _taskscheudulerref)
      (`KismetSystemLibrary.PrintString` (`KismetStringLibrary.Concat_StrStr` "job count:" (`KismetStringLibrary.Conv_IntToString` (`KismetArrayLibrary.Array_Length` (`/Game/Farm_Refactor/Mangers/BP_TaskScheduler.JobQueue` _taskscheudulerref))))))))

(fn `UserConstructionScript`)