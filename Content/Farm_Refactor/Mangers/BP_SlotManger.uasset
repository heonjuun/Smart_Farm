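; BP_SlotManger is a manager Blueprint that keeps a registry of slots for the farm system.
; RegisterSlot adds valid, unique slots to RegisteredSlots and prints a debug message.
; GetSlotByAddress linearly searches that array for matching floor, shelf and slot IDs, storing any match in locals.
; As written, its return sets Found to true regardless of the result and does not pass out the matched slot.
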(fn `GetSlotByAddress`
  (params (InAddress :type "/Game/Farm_Refactor/Data/Struct/ST_SlotAddressRow Structure"))
  (returns (FoundSlot :type "/Game/Farm_Refactor/Slots/BP_PlantSlot Object Reference") (bFound :type Boolean))
  (locals (LocalFoundSlot :type "/Game/Farm_Refactor/Slots/BP_PlantSlot Object Reference") (LocalFound :type Boolean))
  (for _array_element (`self.RegisteredSlots`)
    (bind (_floorid _shelfid _slotid) (break `/Game/Farm_Refactor/Data/Struct/ST_SlotAddressRow` (`/Game/Farm_Refactor/Slots/BP_PlantSlot.SlotAddress` _array_element)))
    (if (and (== InAddress_FloorId_6_2B87F1824A92988B91E9BD8CD431B6AA _floorid) (== InAddress_ShelfId_7_CFE76FE74A69B24523CBFCBC9EAE4B9B _shelfid) (== InAddress_SlotId_8_6BA64B8643A4E049FB8BD399DC3C3F01 _slotid))
      (set `local.LocalFoundSlot` _array_element)
      (set `local.LocalFound` true)
      (break)))
  (return null true))

(fn `RegisterSlot`
  (params (InSlot :type "/Game/Farm_Refactor/Slots/BP_PlantSlot Object Reference"))
  (`/Engine/EditorBlueprintResources/StandardMacros.IsValid` InSlot
    (:`Is Valid`
      (if (not (`KismetArrayLibrary.Array_Contains` (`self.RegisteredSlots`) InSlot))
        (`KismetArrayLibrary.Array_Add` (`self.RegisteredSlots`) InSlot)
        (`KismetSystemLibrary.PrintString` "slot registerd")))))

(fn `UserConstructionScript`)