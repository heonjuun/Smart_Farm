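; Base farm crop actor that can be planted, watered, grown through three mesh stages and harvested, with a tomato mesh at the final stage.
; BeginPlay loads meshes and tuning from a DataTable row; PlantSeed changes the row name without reloading.
; A one-second timer drains water and adds growth unless water falls below a hard-coded 0.3, ignoring the loaded threshold.
; UpdateCropStatusUI writes crop state to a widget component.
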(event `self.ReceiveBeginPlay`
  (`self.LoadCropDefinition`)
  (set `self.CurrentStage` 1)
  (set `self.GrowthPoint` 0.0)
  (set `self.bReadyToHarvest` false)
  (set `self.bNeedWater` false)
  (`self.ApplyStageVisual` 1)
  (`SceneComponent.SetVisibility` (`self.TomatoMesh`) false false)
  (`KismetSystemLibrary.K2_SetTimer` null "UpdateCropGrowth" 1.0 true))

(fn `ApplyStageVisual`
  (params (InStage :type Integer))
  (switch `int` InStage
    (:`1`
      (`StaticMeshComponent.SetStaticMesh` (`self.PlantMesh`) (`self.Stage1`))
      (`SceneComponent.SetVisibility` (`self.TomatoMesh`) false false)
      (set `self.bReadyToHarvest` false)
      (`KismetSystemLibrary.PrintString` "Lv1"))
    (:`2`
      (`StaticMeshComponent.SetStaticMesh` (`self.PlantMesh`) (`self.Stage2`))
      (`SceneComponent.SetVisibility` (`self.TomatoMesh`) false false)
      (set `self.bReadyToHarvest` false)
      (`KismetSystemLibrary.PrintString` "Lv2" true true (struct :`G` 0.66 :`B` 1.0 :`A` 1.0) 222.0))
    (:`3`
      (`StaticMeshComponent.SetStaticMesh` (`self.PlantMesh`) (`self.Stage3`))
      (`StaticMeshComponent.SetStaticMesh` (`self.TomatoMesh`) (`self.Stage3Tomato`))
      (`SceneComponent.SetVisibility` (`self.TomatoMesh`) true false)
      (set `self.bReadyToHarvest` true)
      (set `self.bNeedWater` false)
      (`KismetSystemLibrary.PrintString` "Lv3" true true (struct :`G` 0.66 :`B` 1.0 :`A` 1.0) 22.0))))

(fn `ApplyWater`
  (params (WaterAmount :type "Float (double-precision)"))
  (set `self.WaterLevel` (`KismetMathLibrary.FClamp` (+ WaterAmount (`self.WaterLevel`))))
  (`self.UpdateNeedWaterState`))

(fn `CheckStageUp`
  (if (>= (`self.GrowthPoint`) (`self.Stage3RequiredPoint`))
    (set `self.CurrentStage` 3)
    (`self.ApplyStageVisual` 3)
    (elif (>= (`self.GrowthPoint`) (`self.Stage2RequiredPoint`))
      (set `self.CurrentStage` 2)
      (`self.ApplyStageVisual` 2)
      (elif (<= (`self.GrowthPoint`) 1.0)
        (set `self.CurrentStage` 1)
        (`self.ApplyStageVisual` 1)))))

(fn `HarvestCrop`
  (if (`self.bReadyToHarvest`)
    (set `self.bIsPlanted` false)
    (set `self.CurrentStage` 0)
    (set `self.GrowthPoint` 0.0)
    (set `self.bReadyToHarvest` false)
    (set `self.WaterLevel` 0.0)
    (`self.UpdateNeedWaterState`)
    (set `self.bNeedWater` false)
    (`SceneComponent.SetVisibility` (`self.PlantMesh`) false false)
    (`SceneComponent.SetVisibility` (`self.TomatoMesh`) false false)))

(fn `LoadCropDefinition`
  (`/Engine/EditorBlueprintResources/StandardMacros.IsValid` (`self.CropDefinitionTable`)
    (:`Is Valid`
      (bind _returnvalue (`|GetDataTableRow` (`self.CropDefinitionTable`) (`self.CurrentCropRowName`))
        (:`then`
          (set `self.CropDefinition` _returnvalue)
          (bind (_cropname _stage1mesh _stage2mesh _stage3mesh _tomatomesh _growrate _stage2requiredpoint _stage3requiredpoint _harvestgrowpoint _waterconsumerate _waterneedthreshold _watertargetlevel _seedinitialwaterlevel _seedneedwater) (break `/Game/Farm_Refactor/Data/Struct/ST_CropDefinitionRow` _returnvalue))
          (set `self.Stage1` _stage1mesh)
          (set `self.Stage2` _stage2mesh)
          (set `self.Stage3` _stage3mesh)
          (set `self.Stage3Tomato` _tomatomesh)
          (set `self.GrowthRate` _growrate)
          (set `self.Stage2RequiredPoint` _stage2requiredpoint)
          (set `self.Stage3RequiredPoint` _stage3requiredpoint)
          (set `self.HarvestGrowPoint` _harvestgrowpoint)
          (set `self.WaterConsumRate` _waterconsumerate)
          (set `self.WaterThresHold` _waterneedthreshold)
          (set `self.WaterLevel` _watertargetlevel)
          (set `self.bNeedWater` _seedneedwater))))))

(fn `PlantCrop`
  (set `self.CurrentStage` 1)
  (set `self.GrowthPoint` 0.0)
  (set `self.bReadyToHarvest` false)
  (set `self.bNeedWater` false)
  (set `self.WaterLevel` 0.5)
  (`self.ApplyStageVisual` 1))

(fn `PlantSeed`
  (params (InCropRowName :type Name))
  (if (not (`self.bIsPlanted`))
    (set `self.CurrentCropRowName` InCropRowName)
    (set `self.bIsPlanted` true)
    (set `self.GrowthPoint` 0.0)
    (set `self.bReadyToHarvest` false)
    (set `self.WaterLevel` (`self.SeedInitialWaterLevel`))
    (set `self.bNeedWater` (`self.SeedNeedWater`))
    (`SceneComponent.SetVisibility` (`self.PlantMesh`) true false)
    (`SceneComponent.SetVisibility` (`self.TomatoMesh`) false false)
    (`self.ApplyStageVisual` 1)))

(fn `UpdateCropGrowth`
  (if (`self.bIsPlanted`)
    (if (not (`self.bReadyToHarvest`))
      (set `self.WaterLevel` (`KismetMathLibrary.FClamp` (- (`self.WaterLevel`) (`self.WaterConsumRate`))))
      (`self.UpdateNeedWaterState`)
      (if (not (`self.bNeedWater`))
        (set `self.GrowthPoint` (`KismetMathLibrary.FClamp` (+ (`self.GrowthPoint`) (`self.GrowthRate`)) 0.0 (`self.HarvestGrowPoint`)))
        (`self.CheckStageUp`)))))

(fn `UpdateCropStatusUI`
  (bind _aswbp_crop_status (cast `/Game/Farm_Refactor/UI/WBP_CropStatus` (`WidgetComponent.GetUserWidgetObject` (`self.CropStatusWidget`))))
  (`TextBlock.SetText` (`/Game/Farm_Refactor/UI/WBP_CropStatus.Txt_CropName` _aswbp_crop_status) (`|FormatText` "CropName:{cropname}" (`.Cropname_2_B7DF4F544DB256EF6BF8BD9835EFF21F` (break `/Game/Farm_Refactor/Data/Struct/ST_CropDefinitionRow` (`self.CropDefinition`)))))
  (if (`self.bIsPlanted`)
    (bind _txt_stage (`/Game/Farm_Refactor/UI/WBP_CropStatus.Txt_Stage` _aswbp_crop_status))
    (`TextBlock.SetText` _txt_stage (`|FormatText` "Stage:{stage}" (`self.CurrentStage`)))
    (else
      (`TextBlock.SetText` _txt_stage (`|FormatText` "Stage:0"))))
  (`TextBlock.SetText` (`/Game/Farm_Refactor/UI/WBP_CropStatus.Txt_Water` _aswbp_crop_status) (`|FormatText` "Water:{stage}%" (`self.WaterLevel`)))
  (`TextBlock.SetText` (`/Game/Farm_Refactor/UI/WBP_CropStatus.Txt_Growth` _aswbp_crop_status) (`|FormatText` "Growth:{growth}" (`self.GrowthPoint`))))

(fn `UpdateNeedWaterState`
  (if (< (`self.WaterLevel`) 0.3)
    (set `self.bNeedWater` true)
    (else
      (set `self.bNeedWater` false))))

(fn `UserConstructionScript`)