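; BP_HarvestStorage is a farm storage actor that counts harvested crops and displays them as physical items.
; AddHarvestCount and AddHarvestItem raise one shared total and refresh the WBP_HarvestCount widget on its widget component.
; AddHarvestItem also looks up the crop in DT_CropDefinition and spawns BP_StoredCropItem actors with that crop's mesh.
; Items appear above StoredItemOrigin, spaced along world X by the stored count, with debug prints left in.
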(event `self.ReceiveBeginPlay`
  (`self.UpdateHarvestUI`))

(fn `AddHarvestCount`
  (params (Amount :type Integer))
  (set `self.HarvestCount` (+ Amount (`self.HarvestCount`)))
  (`self.UpdateHarvestUI`))

(fn `AddHarvestItem`
  (params (CropRowName :type Name) (Amount :type Integer))
  (set `self.HarvestCount` (+ (`self.HarvestCount`) Amount))
  (`self.UpdateHarvestUI`)
  (`self.SpawnStoredCropItems` CropRowName Amount))

(fn `SpawnStoredCropItems`
  (params (CropName :type Name) (Amount :type Integer))
  (`KismetSystemLibrary.PrintString` (`KismetTextLibrary.Conv_TextToString` (`|FormatText` "스폰스토어드크랍아이템:{0}" CropName)) true true (struct :`G` 0.66 :`B` 1.0 :`A` 1.0) 22.0 CropName)
  (`KismetSystemLibrary.PrintString` (`KismetTextLibrary.Conv_TextToString` (`|FormatText` "어마운트:{0}" Amount)) true true (struct :`G` 0.66 :`B` 1.0 :`A` 1.0) 22.0)
  (bind _returnvalue (`|GetDataTableRow` "/Game/Farm_Refactor/Data/DataTable/DT_CropDefinition.DT_CropDefinition" CropName)
    (:`then`
      (for _ (range Amount)
        (bind _returnvalue_2 (`|SpawnActorFromClass` "/Game/Farm_Refactor/Crops/BP_StoredCropItem.BP_StoredCropItem_C" (`KismetMathLibrary.MakeTransform` (+ (`SceneComponent.K2_GetComponentLocation` (`self.StoredItemOrigin`)) (`KismetMathLibrary.MakeVector` (* (`KismetMathLibrary.Conv_IntToDouble` (`KismetArrayLibrary.Array_Length` (`self.StoredCropItems`))) (`self.CropItemSpacing`)) 0.0 200.0)) (`SceneComponent.K2_GetComponentRotation` (`self.StoredItemOrigin`))) "AlwaysSpawn" "MultiplyWithRoot" null null))
        (`/Engine/EditorBlueprintResources/StandardMacros.IsValid` _returnvalue_2
          (:`Is Valid`
            (bind (_cropname _stage1mesh _stage2mesh _stage3mesh _tomatomesh _growrate _stage2requiredpoint _stage3requiredpoint _harvestgrowpoint _waterconsumerate _waterneedthreshold _watertargetlevel _seedinitialwaterlevel _seedneedwater _mintemparature _maxtemparature _minhumidity _maxhumidity _minc02 _maxco2 _requirelight _storeditemmesh) (break `/Game/Farm_Refactor/Data/Struct/ST_CropDefinitionRow` _returnvalue))
            (`/Game/Farm_Refactor/Crops/BP_StoredCropItem.InitStoredItem` _returnvalue_2 (`KismetStringLibrary.Conv_StringToName` _cropname) _storeditemmesh)
            (`KismetArrayLibrary.Array_Add` (`self.StoredCropItems`) _returnvalue_2)))))
    (:`RowNotFound`
      (`KismetSystemLibrary.PrintString` "harvest stroage not found" true true (struct :`G` 0.66 :`B` 1.0 :`A` 1.0) 22220.0))))

(fn `UpdateHarvestUI`
  (bind _aswbp_harvest_count (cast `/Game/Farm_Refactor/UI/WBP_HarvestCount` (`WidgetComponent.GetUserWidgetObject` (`self.HarvestCountWidget`))))
  (`TextBlock.SetText` (`/Game/Farm_Refactor/UI/WBP_HarvestCount.Txt_HarvestCount` _aswbp_harvest_count) (`|FormatText` "HarvestCount:{Count}" (`KismetTextLibrary.Conv_IntToText` (`self.HarvestCount`)))))

(fn `UserConstructionScript`)