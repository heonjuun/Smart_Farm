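; Procedural farm shelf actor that builds tiered racks with pots and LEDs and can host crops.
; The construction script rebuilds three instanced mesh components from count and spacing variables, placing pots at two X positions and appending farm Slots inside the nested LED loop.
; SpawnCrop spawns BP_CropBase for an unoccupied slot at the last stored PotTransForm, rather than that slot's transform.
; ClearCrop is an empty stub.
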(fn `ClearCrop`)

(fn `SpawnCrop`
  (params (SlotIndex :type Integer))
  (bind (_output_address _output_pottransform _output_worktransform _output_croprowname _output_boccupied) (break `/Game/Farm_Refactor/Data/Struct/ST_FarmSlot` (`|GetArrayItem` (`self.Slots`) SlotIndex)))
  (if (not _output_boccupied)
    (`|SpawnActorFromClass` "/Game/Farm_Refactor/Crops/BP_CropBase.BP_CropBase_C" (`self.PotTransForm`) "Undefined" "MultiplyWithRoot" null self SlotIndex null)))

(fn `UserConstructionScript`
  (bind _returnvalue (`KismetMathLibrary.MakeTransform` (`KismetMathLibrary.MakeVector` (`self.StartX`) 0.0 (`self.Floor`))))
  (`InstancedStaticMeshComponent.ClearInstances` (`self.PotISM`))
  (`InstancedStaticMeshComponent.ClearInstances` (`self.ShelfISM`))
  (`InstancedStaticMeshComponent.ClearInstances` (`self.LEDISM`))
  (`KismetArrayLibrary.Array_Clear` (`self.Slots`))
  (for _index (range (`self.TierCount`))
    (`InstancedStaticMeshComponent.AddInstance` (`self.ShelfISM`) (`KismetMathLibrary.MakeTransform` (`KismetMathLibrary.MakeVector` 0.0 0.0 (* _index (`self.TierHeight`)))) false)
    (for _index_2 (range (`self.PotsPerRow`))
      (for _index_3 (range (`self.ShelfCount`))
        (bind _returnvalue_2 (`KismetMathLibrary.Conv_IntToDouble` (* _index_3 (`self.ShelfHeight`))))
        (set `self.Floor` _returnvalue_2)
        (`|ExecutionSequence`
          (:`then_0`
            (bind _returnvalue_3 (- (* _index_2 (`self.PotSpacing`)) (`self.PotY`)))
            (`InstancedStaticMeshComponent.AddInstance` (`self.PotISM`) (`KismetMathLibrary.MakeTransform` (`KismetMathLibrary.MakeVector` (`self.StartX`) _returnvalue_3 _returnvalue_2)) false))
          (:`then_1`
            (`InstancedStaticMeshComponent.AddInstance` (`self.PotISM`) (`KismetMathLibrary.MakeTransform` (`KismetMathLibrary.MakeVector` (`self.EndX`) _returnvalue_3 _returnvalue_2)) false)))
        (for _index_4 (range (`self.LEDsPerTier`))
          (`InstancedStaticMeshComponent.AddInstance` (`self.LEDISM`) (`KismetMathLibrary.MakeTransform` (`KismetMathLibrary.MakeVector` 0.0 0.0 (* _index_4 (`self.LEDHeight`))) (`KismetMathLibrary.MakeRotator` 0.0 0.0 (`self.LEDYaw`))) false)
          (`|ExecutionSequence`
            (:`then_0`
              (set `self.PotTransForm` _returnvalue)
              (`KismetArrayLibrary.Array_Add` (`self.Slots`) (make `/Game/Farm_Refactor/Data/Struct/ST_FarmSlot` (make `/Game/Farm_Refactor/Data/Struct/ST_SlotAddressRow` (`KismetMathLibrary.FTrunc` (`self.Floor`)) (`self.ShelfID`) (`KismetArrayLibrary.Array_Length` (`self.Slots`))) _returnvalue (`KismetMathLibrary.MakeTransform` (`KismetMathLibrary.MakeVector` (`self.StartX`) (`self.WorkFrontY`))) "None" false null)))))))))