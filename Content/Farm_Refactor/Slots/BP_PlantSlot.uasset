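; BP_PlantSlot is a farm slot that holds a single crop reference and tracks whether it is occupied.
; On BeginPlay it reads its default crop from the hardcoded "Tomato" row of DT_SlotDefinition, then registers with BP_SlotManger.
; SpawnCrop spawns a BP_CropBase at CropPoint, links crop and slot to each other through SetCrop, and plants the requested seed row.
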(event `self.ReceiveBeginPlay`
  (bind _returnvalue (`|GetDataTableRow` "/Game/Farm_Refactor/Data/DataTable/DT_SlotDefinition.DT_SlotDefinition" "Tomato")
    (:`then`
      (set `self.DefaultCropRowName` (break `/Game/Farm_Refactor/Data/Struct/ST_SlotDefinitionRow` _returnvalue))
      (bind _returnvalue_2 (`GameplayStatics.GetActorOfClass` "/Game/Farm_Refactor/Managers/BP_SlotManger.BP_SlotManger_C"))
      (bind _asbp_slot_manger (cast `/Game/Farm_Refactor/Managers/BP_SlotManger` _returnvalue_2))
      (`/Game/Farm_Refactor/Managers/BP_SlotManger.RegisterSlot` _asbp_slot_manger self))))

(fn `SetCrop`
  (params (InCrop :type "/Game/Farm_Refactor/Crops/BP_CropBase Object Reference"))
  (set `self.CropRef` InCrop)
  (bind _output_get (set `/Game/Farm_Refactor/Crops/BP_CropBase.OwnerSlot` self (`self.CropRef`)))
  (`/Engine/EditorBlueprintResources/StandardMacros.IsValid` _output_get
    (:`Is Valid`
      (set `self.bOccupied` true))
    (:`Is Not Valid`
      (set `self.bOccupied` false))))

(fn `SpawnCrop`
  (params (InCropRowName :type Name))
  (bind _returnvalue (`|SpawnActorFromClass` "/Game/Farm_Refactor/Crops/BP_CropBase.BP_CropBase_C" (`KismetMathLibrary.MakeTransform` (`SceneComponent.K2_GetComponentLocation` (`self.CropPoint`))) "AlwaysSpawn" "MultiplyWithRoot" null self null))
  (`self.SetCrop` _returnvalue)
  (`/Game/Farm_Refactor/Crops/BP_CropBase.PlantSeed` _returnvalue InCropRowName))

(fn `UserConstructionScript`)